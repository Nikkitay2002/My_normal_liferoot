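; BP_FinishPoint is a finish-point Blueprint that shows a collect-point widget whose appearance follows its current tag.
; ChangeState stores the new tag and uses it as the row name to look up DT_Points.
; When the row is found, it applies that row's texture, name and color to the WB_CollectPoint in the Point widget component and passes the tag on.
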(event `ChangeState`
  (params (NewTag :type Name))
  (bind _mytag (`self.MyTag`))
  (set `self.MyTag` NewTag)
  (bind _aswb_collect_point (cast `/Game/Items/Points/Widgets/WB_CollectPoint` (`WidgetComponent.GetWidget` (`self.Point`))))
  (bind _returnvalue (`|GetDataTableRow` "/Game/Items/Points/DT_Points.DT_Points" _mytag)
    (:`then`
      (bind (_name _texture _color) (break `/Game/Items/Points/Points_Structure` _returnvalue))
      (`Image.SetBrushFromTexture` (`/Game/Items/Points/Widgets/WB_CollectPoint.Image_17` _aswb_collect_point) _texture false)
      (bind _name_2 (`/Game/Items/Points/Widgets/WB_CollectPoint.Name` _aswb_collect_point))
      (set `TextBlock.ColorAndOpacity` _color _name_2)
      (`TextBlock.SetText` _name_2 _name)
      (set `/Game/Items/Points/Widgets/WB_CollectPoint.Tag` _mytag _aswb_collect_point))))

(fn `UserConstructionScript`
  (`parent.UserConstructionScript`))