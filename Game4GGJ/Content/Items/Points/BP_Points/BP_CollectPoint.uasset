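; BP_CollectPoint is a collect point actor that shows a widget marker configured per point type.
; On BeginPlay it hides the Point widget and uses MyTag to look up a DT_Points row, which fills WB_CollectPoint's icon, name text and color, and the tag is passed along.
; SetVisible reveals a hidden marker temporarily, then hides it again after a fixed delay.
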(event `self.ReceiveBeginPlay`
  (bind _point (`self.Point`))
  (bind _mytag (`self.MyTag`))
  (`SceneComponent.SetVisibility` _point false false)
  (bind _aswb_collect_point (cast `/Game/Items/Points/Widgets/WB_CollectPoint` (`WidgetComponent.GetWidget` _point)))
  (bind _returnvalue (`|GetDataTableRow` "/Game/Items/Points/DT_Points.DT_Points" _mytag)
    (:`then`
      (bind (_name _texture _color) (break `/Game/Items/Points/Points_Structure` _returnvalue))
      (`Image.SetBrushFromTexture` (`/Game/Items/Points/Widgets/WB_CollectPoint.Image_17` _aswb_collect_point) _texture false)
      (bind _name_2 (`/Game/Items/Points/Widgets/WB_CollectPoint.Name` _aswb_collect_point))
      (set `TextBlock.ColorAndOpacity` _color _name_2)
      (`TextBlock.SetText` _name_2 _name)
      (set `/Game/Items/Points/Widgets/WB_CollectPoint.Tag` _mytag _aswb_collect_point))))

(event `SetVisible`
  (bind _point (`self.Point`))
  (if (not (`SceneComponent.bVisible` _point))
    (`SceneComponent.SetVisibility` _point true false)
    (`KismetSystemLibrary.Delay` 10.0)
    (`SceneComponent.SetVisibility` _point false false)))

(fn `UserConstructionScript`)