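; BP_File is a collectable file that the main character picks up by overlapping its capsule, unlocking the level's exit when it is the last one.
; Pickup shows a HUD message with the level number parsed from the level name, plays a sound and destroys the BP_CollectPoint sharing its Id.
; It counts remaining files; the last frees End_Platform, opens BP_FinishPoint and toggles the BP_NextLevel_col lock.
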(event `self.Capsule.OnComponentBeginOverlap`
  (params (OverlappedComponent :type "PrimitiveComponent Object Reference") (OtherActor :type "Actor Object Reference") (OtherComp :type "PrimitiveComponent Object Reference") (OtherBodyIndex :type Integer) (bFromSweep :type Boolean) (SweepResult :type "HitResult Structure (by ref)"))
  (if (`KismetMathLibrary.ClassIsChildOf` (`GameplayStatics.GetObjectClass` OtherActor) "/Game/FirstPerson/Blueprints/BP_MC_Father.BP_MC_Father_C")
    (message `/Game/Widgets/I_shizoid.FilesPickUp` (`/Game/FirstPerson/Blueprints/BP_MainCharacter.HUDStats` (`self.As BP Main Character`)) (`KismetStringLibrary.Conv_StringToInt` (`self.CurrentLevel`)))
    (`GameplayStatics.PlaySound2D` "/Game/Audio/Effects/Collectables_pick_up.Collectables_pick_up" 1.0 1.0 0.0 null null)
    ;[1 0 0.04385] Destroy File and Point
    (bind _outactors (`GameplayStatics.GetAllActorsOfClass` "BP_File_C"))
    (bind _outactors_2 (`GameplayStatics.GetAllActorsOfClass` "/Game/Items/Points/BP_Points/BP_CollectPoint.BP_CollectPoint_C"))
    (for _array_element _outactors_2
      (if (== (`self.id`) (`/Game/Items/Points/BP_Points/BP_CollectPoint.id` _array_element))
        (`self.K2_DestroyActor` _array_element)))
    ;[0.1536 1 0.002934] Open Level
    (if (== (`KismetArrayLibrary.Array_Length` _outactors) 1)
      (bind _returnvalue (`GameplayStatics.GetActorOfClass` "/Game/Nikitay/Meshes/End_Platform.End_Platform_C"))
      (`/Game/Nikitay/Meshes/End_Platform.FreeToFinish` _returnvalue)
      (bind _returnvalue_2 (`GameplayStatics.GetActorOfClass` "/Game/Items/Points/BP_Points/BP_FinishPoint.BP_FinishPoint_C"))
      (`/Engine/EditorBlueprintResources/StandardMacros.IsValid` _returnvalue_2
        (:`Is Valid`
          (`/Game/Items/Points/BP_Points/BP_FinishPoint.ChangeState` _returnvalue_2 "FinishPointOpen")
          (bind _returnvalue_3 (`GameplayStatics.GetActorOfClass` "/Game/Nikitay/Materials/test/LVL1/BP_NextLevel_col.BP_NextLevel_col_C"))
          (`/Engine/EditorBlueprintResources/StandardMacros.IsValid` _returnvalue_3
            (:`Is Valid`
              (`/Game/Nikitay/Materials/test/LVL1/BP_NextLevel_col.changeLock` _returnvalue_3)
              (`self.K2_DestroyActor`)
              (`self.K2_DestroyActor`)))))
      (else
        (`self.K2_DestroyActor`)))))

(event `self.ReceiveBeginPlay`
  (bind _asbp_main_character (cast `/Game/FirstPerson/Blueprints/BP_MainCharacter` (`GameplayStatics.GetPlayerCharacter` 0)))
  (set `self.As BP Main Character` _asbp_main_character)
  (bind _returnvalue (`GameplayStatics.GetCurrentLevelName` true))
  (set `self.CurrentLevel` (`.RightS` (`KismetStringLibrary.Split` _returnvalue "lvl"))))

(fn `UserConstructionScript`)