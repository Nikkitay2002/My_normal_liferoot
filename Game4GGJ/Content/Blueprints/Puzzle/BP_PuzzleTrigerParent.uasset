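; BP_PuzzleTrigerParent is a pressure-button trigger for puzzles, named as a parent class, that reacts to BP_MainCharacter entering or leaving its Box.
; Overlap begin and end set IsButtonPressed on and off, play a sound at the root and print a debug string.
; On press it can also spawn a configurable ActorClass at ActorTransform when IsNeedToCreateActor is set, with no guard against repeated spawns.
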(event `self.Box.OnComponentBeginOverlap`
  (params (OverlappedComponent :type "PrimitiveComponent Object Reference") (OtherActor :type "Actor Object Reference") (OtherComp :type "PrimitiveComponent Object Reference") (OtherBodyIndex :type Integer) (bFromSweep :type Boolean) (SweepResult :type "HitResult Structure (by ref)"))
  (bind _asbp_main_character (cast `/Game/FirstPerson/Blueprints/BP_MainCharacter` OtherActor))
  (`KismetSystemLibrary.PrintString` (`KismetStringLibrary.Concat_StrStr` (`KismetSystemLibrary.GetDisplayName` _asbp_main_character) ": 1") true false (struct :`G` 1.0 :`A` 1.0) 5.0)
  (`GameplayStatics.PlaySoundAtLocation` null (`SceneComponent.K2_GetComponentLocation` (`self.DefaultSceneRoot`)) (struct) 1.0 1.0 0.0 null null null null)
  (set `self.IsButtonPressed?` true)
  (if (`self.IsNeedToCreateActor?`)
    (`|SpawnActorFromClass` (`self.ActorClass`) (`self.ActorTransform`) "Undefined" "OverrideRootScale" null null)))

(event `self.Box.OnComponentEndOverlap`
  (params (OverlappedComponent :type "PrimitiveComponent Object Reference") (OtherActor :type "Actor Object Reference") (OtherComp :type "PrimitiveComponent Object Reference") (OtherBodyIndex :type Integer))
  (bind _asbp_main_character (cast `/Game/FirstPerson/Blueprints/BP_MainCharacter` OtherActor))
  (`KismetSystemLibrary.PrintString` (`KismetStringLibrary.Concat_StrStr` (`KismetSystemLibrary.GetDisplayName` _asbp_main_character) ": 0") true false (struct :`R` 1.0 :`A` 1.0) 5.0)
  (`GameplayStatics.PlaySoundAtLocation` null (`SceneComponent.K2_GetComponentLocation` (`self.DefaultSceneRoot`)) (struct) 1.0 1.0 0.0 null null null null)
  (set `self.IsButtonPressed?` false))

(fn `UserConstructionScript`)