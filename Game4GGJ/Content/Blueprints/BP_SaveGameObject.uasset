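; Save game object that stores which levels are locked and supplies that state to the HUD's level buttons.
; InitializeButton looks up a level's lock flag by ID in the IsLevelLocked struct array and caches the HUD reference.
; SetLevelLocked rewrites the matching entry and pushes the new state to HUD buttons through SetBlocking.
; AddButtonRef separately adds unique entries to a ButtonsRef array.
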(fn `AddButtonRef`
  (params (NewItem :type "/Game/UI/MainMenu/UI_Elements/MainMenuButton Object Reference (by ref)"))
  (returns (ArrayIndex :type Integer))
  (bind _returnvalue (`KismetArrayLibrary.Array_AddUnique` (`self.ButtonsRef`)))
  (return _returnvalue))

(fn `InitializeButton`
  (params (LevelId :type "/Game/UI/MainMenu/UI_Elements/Buttons_Enum Enum" :default "NewEnumerator0") (HUD :type "/Game/UI/MainMenu/MainMenu_Scene/MainMenuHUD Object Reference"))
  (returns (IsLocked :type Boolean))
  (bind _islevellocked (`self.IsLevelLocked`))
  (for (_array_element _array_index) _islevellocked
    (if (`|EnumEquality` (`.LevelID_10_9DDE30864990996D031B148F583E35AF` (break `/Game/UI/MainMenu/UI_Elements/IsLevelLocked` _array_element)) LevelId)
      (break)))
  (set `self.HUD` HUD)
  (return (`.IsLocked_1_EFD4910746C387B08DFCB5A954273791` (break `/Game/UI/MainMenu/UI_Elements/IsLevelLocked` (`|GetArrayItem` _islevellocked _array_index)))))

(fn `Set Level Locked`
  (params (LevelId :type "/Game/UI/MainMenu/UI_Elements/Buttons_Enum Enum" :default "NewEnumerator0") (IsLocked :type Boolean) (HUD_TOCHNO :type "/Game/UI/MainMenu/MainMenu_Scene/MainMenuHUD Object Reference"))
  (bind _islevellocked (`self.IsLevelLocked`))
  (bind _buttonsarray (`/Game/UI/MainMenu/MainMenu_Scene/MainMenuHUD.ButtonsArray` (`self.HUD`)))
  (set `self.HUD` HUD_TOCHNO)
  (for (_array_element _array_index) _islevellocked
    (if (`|EnumEquality` (`.LevelID_10_9DDE30864990996D031B148F583E35AF` (break `/Game/UI/MainMenu/UI_Elements/IsLevelLocked` _array_element)) LevelId)
      (break)))
  (`KismetArrayLibrary.Array_Set` _islevellocked _array_index (make `/Game/UI/MainMenu/UI_Elements/IsLevelLocked` IsLocked LevelId))
  (for _ _buttonsarray
    (`/Game/UI/MainMenu/UI_Elements/MainMenuButton.SetBlocking` (`|GetArrayItem` _buttonsarray _array_index) IsLocked)))