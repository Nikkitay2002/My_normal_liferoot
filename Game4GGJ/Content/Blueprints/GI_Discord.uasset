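; Game Instance that shows the game's status as Discord Rich Presence.
; Init creates and initializes a DiscordRpc object with the application ID, and Shutdown clears the presence.
; Setters store the start time and level details without publishing them; the Rich Presence function combines them with a given state and fixed image key, prints the timestamp and pushes the update.
; ChangeState publishes through that function and records the current state.
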(event `self.ReceiveInit`
  (bind _returnvalue (`|GenericCreateObject` "/Script/DiscordRpc.DiscordRpc"))
  (bind _output_get (set `self.DiscordRPC` _returnvalue))
  (`DiscordRpc.Initialize` _output_get (`self.Application Id`) false ""))

(event `self.ReceiveShutdown`
  (`DiscordRpc.ClearPresence` (`self.DiscordRPC`)))

(event `SetMyTime`
  (params (Float :type Integer))
  (set `self.StartTime` Float))

(event `/Game/Blueprints/BPI_GameInstance.SetDetailsLevel`
  (params (Details :type String))
  (set `self.Details NOW` Details))

(fn `ChangeState`
  (params (State :type String))
  (returns (NewParam :type Boolean))
  (bind _returnvalue (`self.Rich Presence` State))
  (set `self.State NOW` State)
  (return _returnvalue))

(fn `Rich Presence`
  (params (State :type String))
  (returns (ReturnValue :type Boolean))
  (bind _discordrpc (`self.DiscordRPC`))
  (bind _returnvalue (+ (`self.StartTime`) 0))
  (`KismetSystemLibrary.PrintString` (`KismetStringLibrary.Conv_IntToString` _returnvalue) true true (struct :`R` 1.0 :`B` 0.006324 :`A` 1.0))
  (bind _structout (setmembers `DiscordRichPresence` :`StructRef` (`DiscordRpc.RichPresence` (`self.DiscordRPC`)) :`state` State :`details` (`self.Details NOW`) :`startTimestamp` _returnvalue :`largeImageKey` "temininotext"))
  (set `DiscordRpc.RichPresence` _structout _discordrpc)
  (`DiscordRpc.UpdatePresence` _discordrpc)
  (return true))

(fn `RichPresence`
  (params (State :type String))
  (returns (ReturnValue :type Boolean))
  (bind _returnvalue (`self.Rich Presence` State))
  (return _returnvalue))

(fn `Set Discord Time`
  (params (StartTime :type String))
  (returns (NewParam :type Boolean))
  (`self.SetMyTime` (`KismetStringLibrary.Conv_StringToInt` StartTime))
  (return false))