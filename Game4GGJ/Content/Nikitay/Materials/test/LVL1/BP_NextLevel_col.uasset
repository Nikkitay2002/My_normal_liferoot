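; BP_NextLevel_col is a level-exit trigger that records progress and opens the next level when the main character enters its box.
; The overlap only acts after changeLock has set CanFinish.
; It asynchronously loads the "Save" slot, first saving the BP_SaveGameObject created at BeginPlay if none exists.
; It then increments the saved Level, saves it back and opens the level named by LevelName.
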(event `changeLock`
  (set `self.canFinish` true))

(event `self.Box.OnComponentBeginOverlap`
  (params (OverlappedComponent :type "PrimitiveComponent Object Reference") (OtherActor :type "Actor Object Reference") (OtherComp :type "PrimitiveComponent Object Reference") (OtherBodyIndex :type Integer) (bFromSweep :type Boolean) (SweepResult :type "HitResult Structure (by ref)"))
  (if (`self.canFinish`)
    (cast `/Game/FirstPerson/Blueprints/BP_MainCharacter` OtherActor)
    (bind _returnvalue (`GameplayStatics.DoesSaveGameExist` "Save"))
    (if (not _returnvalue)
      (`AsyncActionHandleSaveGame.AsyncSaveGameToSlot` (stale `self.ReceiveBeginPlay` _returnvalue) "Save"
        (:`Completed`
          _)))
    (bind _savegame (`AsyncActionHandleSaveGame.AsyncLoadGameFromSlot` "Save")
      (:`Completed`
        (bind _asbp_save_game_object (cast `/Game/Blueprints/BP_SaveGameObject` _savegame))
        (`/Engine/EditorBlueprintResources/StandardMacros.IncrementInt` (`/Game/Blueprints/BP_SaveGameObject.Level` _asbp_save_game_object)
          (:`  `
            (`AsyncActionHandleSaveGame.AsyncSaveGameToSlot` _asbp_save_game_object "Save"
              (:`Completed`
                (`GameplayStatics.OpenLevel` (`self.Level Name`))))))))))

(event `self.ReceiveBeginPlay`
  (bind _returnvalue (`GameplayStatics.CreateSaveGameObject` "/Game/Blueprints/BP_SaveGameObject.BP_SaveGameObject_C")))

(fn `UserConstructionScript`)